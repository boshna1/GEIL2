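; BP_TurretBase_Var1 is a turret variant that configures an inherited turret base Blueprint.
; On BeginPlay it sets fire rate, bullet class (BP_Bullet_Var1) and spin speed, prints a debug message, then calls the parent BeginPlay so the base starts with those values.
; Tick and construction defer entirely to the parent, and the overlap event is disabled.
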(event EventBeginPlay
  (Utilities|FlowControl|Sequence
    (:then_0
      (Variables|Default|SetFireRate 0.2))
    (:then_1
      (Variables|Default|SetBP_BulletBase "/Game/Blueprints/BP_Bullet_Var1.BP_Bullet_Var1_C"))
    (:then_2
      (Variables|Default|SetSpinSpeed 2e+01))
    (:then_3
      (Development|PrintString "var set" true true "(R=0.000000,G=0.660000,B=1.000000,A=1.000000)" 5.0))
    (:then_4
      (|CallParentFunction))))

(event Collision|EventActorBeginOverlap
  (params (OtherActor :type Actor%20Object%20Reference))
  (|CallParentFunction OtherActor) ; This node is disabled and will not be called.\nDrag off pins to build functionality.
)

(event EventTick
  (params (DeltaSeconds :type Float%20%28single-precision%29))
  (|CallParentFunction DeltaSeconds))

(fn ConstructionScript
  (|CallParentFunction))