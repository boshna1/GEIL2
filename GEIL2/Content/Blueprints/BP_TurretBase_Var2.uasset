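; BP_TurretBase_Var2 is a turret variant that configures inherited turret behavior with its own fire rate, bullet class and spin speed.
; On BeginPlay it sets these values, choosing BP_Bullet_Var2 as the bullet, then calls the parent BeginPlay so they are in place before parent startup logic runs.
; The construction script only calls the parent, and the overlap and Tick events are disabled placeholders.
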(event EventBeginPlay
  (Utilities|FlowControl|Sequence
    (:then_0
      (Variables|Default|SetFireRate 0.1))
    (:then_1
      (Variables|Default|SetBP_BulletBase "/Game/Blueprints/BP_Bullet_Var2.BP_Bullet_Var2_C"))
    (:then_2
      (Variables|Default|SetSpinSpeed 5e+01))
    (:then_3
      (|CallParentFunction))))

(event Collision|EventActorBeginOverlap
  (params (OtherActor :type Actor%20Object%20Reference))
  (|CallParentFunction OtherActor) ; This node is disabled and will not be called.\nDrag off pins to build functionality.
)

(event EventTick
  (params (DeltaSeconds :type Float%20%28single-precision%29))
  (|CallParentFunction DeltaSeconds) ; This node is disabled and will not be called.\nDrag off pins to build functionality.
)

(fn ConstructionScript
  (|CallParentFunction))