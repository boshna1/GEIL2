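; Base turret actor that automatically fires bullets on a repeating timer.
; BeginPlay starts looping timers for Shoot and Scan.
; Shoot spawns a bullet at the turret's transform, then blocks firing until a FireRate timer resets CanShoot.
; Scan is a spin step that sets yaw from SpinSpeed, frame delta and current roll rather than current yaw, so rotation does not accumulate.
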(event Custom|Shoot
  (Development|PrintString "shoot fire" true true "(R=0.000000,G=0.660000,B=1.000000,A=1.000000)" 5.0)
  (if (Variables|Default|GetCanShoot)
    (bind _returnvalue (Game|SpawnActorfromClass (Variables|Default|GetBP_BulletBase) (Transformation|GetActorTransform) "Undefined" "MultiplyWithRoot" 0 0))
    (Variables|Default|SetCanShoot false)
    (Utilities|Time|SetTimerbyEvent (delegate Custom|ResetCanShoot) (Variables|Default|GetFireRate))
    (Utilities|Casting|CastToBP_BulletBase _returnvalue)))

(event Custom|ResetCanShoot
  (Variables|Default|SetCanShoot true))

(event Custom|Scan
  (Transformation|SetActorTransform (Math|Transform|MakeTransform (Transformation|GetActorLocation) (Math|Rotator|MakeRotator 0.0 0.0 (+ (* (Utilities|Time|GetWorldDeltaSeconds) (Variables|Default|GetSpinSpeed)) (.Roll (Math|Rotator|BreakRotator (Transformation|GetActorRotation))))))))

(event EventBeginPlay
  (Utilities|FlowControl|Sequence
    (:then_0
      (Variables|Default|SetCanShoot true))
    (:then_1
      (Utilities|Time|SetTimerbyEvent (delegate Custom|Shoot) (Variables|Default|GetFireRate) true)
      (Utilities|Time|SetTimerbyEvent (delegate Custom|Scan) 0.1 true))))

(event Collision|EventActorBeginOverlap
  (params (OtherActor :type Actor%20Object%20Reference)))

(event EventTick
  (params (DeltaSeconds :type Float%20%28single-precision%29)))

(fn ConstructionScript)